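; Player-flyable P-38 aircraft pawn that moves forward every tick, turns on pitch and roll axes, and fires rockets.
; Axis input applies frame-time-scaled local rotation, Boost adds a one-off larger forward input per press, and Fire spawns BP_Rocket at the pawn's transform.
; BeginPlay registers Left and Right with BPRotateSceneComponent.
; The RoatatePropeller function is uncalled here and multiplies its roll by zero.
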(event `self.ReceiveBeginPlay`
  (`KismetArrayLibrary.Array_Add` (`/Game/Blueprints/BP_RotateSceneComponent.SceneComponent` (`self.BP_RotateSceneComponent`)) (`self.Left`))
  (`KismetArrayLibrary.Array_Add` (`/Game/Blueprints/BP_RotateSceneComponent.SceneComponent` (`self.BP_RotateSceneComponent`)) (`self.Right`)))

(event `InputAction|Boost`
  (params (Key :type "Key Structure"))
  ;[1 1 1] Boost
  (:`Pressed`
    (`self.AddMovementInput` (`self.GetActorForwardVector`) 10.0)))

(event `self.ReceiveTick`
  (params (DeltaSeconds :type "Float (single-precision)"))
  (`self.AddMovementInput` (`self.GetActorForwardVector`)))

(event `InputAxis|Pitch`
  (params (AxisValue :type "Float (single-precision)"))
  (`self.K2_AddActorLocalRotation` (`KismetMathLibrary.MakeRotator` 0.0 (* AxisValue (`self.RotateSpeed`) (`GameplayStatics.GetWorldDeltaSeconds`)))))

(event `InputAxis|Roll`
  (params (AxisValue :type "Float (single-precision)"))
  (`self.K2_AddActorLocalRotation` (`KismetMathLibrary.MakeRotator` (* AxisValue (`self.RotateSpeed`) (`GameplayStatics.GetWorldDeltaSeconds`)))))

(event `InputAction|Fire`
  (params (Key :type "Key Structure"))
  (:`Pressed`
    (`|SpawnActorFromClass` "/Game/Blueprints/BP_Rocket.BP_Rocket_C" (`self.GetTransform`) "Undefined" "MultiplyWithRoot" null null)))

(fn `RoatatePropeller`
  (params (where :type "SceneComponent Object Reference"))
  ;[1 1 1] 프로펠러 속도 함수
  (`SceneComponent.K2_AddLocalRotation` where (`KismetMathLibrary.MakeRotator` (* (`GameplayStatics.GetWorldDeltaSeconds`) 0.0)) false false))

(fn `UserConstructionScript`)