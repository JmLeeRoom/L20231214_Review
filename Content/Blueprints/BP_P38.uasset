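; BP_P38 is a P-38 aircraft Blueprint with spinning propeller components.
; On BeginPlay it registers its Left and Right components in the BPRotateSceneComponent's array, presumably handing their rotation to that reusable component.
; A RoatatePropeller function can roll a given component at a frame-rate-independent PropellerRotationSpeed, but nothing in this graph calls it.
; Tick, overlap and construction logic are empty.
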(event `self.ReceiveBeginPlay`
  (`KismetArrayLibrary.Array_Add` (`/Game/Blueprints/BP_RotateSceneComponent.SceneComponent` (`self.BP_RotateSceneComponent`)) (`self.Left`))
  (`KismetArrayLibrary.Array_Add` (`/Game/Blueprints/BP_RotateSceneComponent.SceneComponent` (`self.BP_RotateSceneComponent`)) (`self.Right`)))

(fn `RoatatePropeller`
  (params (where :type "SceneComponent Object Reference"))
  ;[1 1 1] 프로펠러 속도 함수
  (`SceneComponent.K2_AddLocalRotation` where (`KismetMathLibrary.MakeRotator` (* (`GameplayStatics.GetWorldDeltaSeconds`) (`self.PropellerRotationSpeed`))) false false))

(fn `UserConstructionScript`)